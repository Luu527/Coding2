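; BP_MachineGun is a machine gun pickup that can be carried, used and dropped.
; PickUp prints a message, attaches the gun to the given skeletal mesh's hand_r socket and disables Body collision.
; UsePrimary only prints placeholder firing text, with no shooting logic.
; Drop detaches the gun, restores collision and briefly simulates physics on Body, switching it off after a fixed delay.
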(event `/Game/Blueprints/Coding2/BPI_Item.PickUp`
  (params (SkeletalMesh :type "SkeletalMeshComponent Object Reference"))
  ; pickUpFunction
  (`KismetSystemLibrary.PrintText` (`|FormatText` "{Name} is getting picked up and attached to {mesh} " "Machine Gun" SkeletalMesh) true true (struct :`R` 1.0 :`G` 0.140625 :`B` 0.24753 :`A` 1.0) 5.0)
  (`self.K2_AttachToComponent` SkeletalMesh "hand_r" "SnapToTarget" "SnapToTarget" "KeepRelative")
  (`PrimitiveComponent.SetCollisionEnabled` (`self.Body`) "NoCollision"))

(event `/Game/Blueprints/Coding2/BPI_Item.UsePrimary`
  (`KismetSystemLibrary.PrintText` "pew pew pew"))

(event `/Game/Blueprints/Coding2/BPI_Item.Drop`
  (`self.K2_DetachFromActor` "KeepWorld" "KeepWorld")
  (`PrimitiveComponent.SetSimulatePhysics` (`self.Body`) true)
  (`PrimitiveComponent.SetCollisionEnabled` (`self.Body`) "QueryAndPhysics")
  (`KismetSystemLibrary.Delay` 2.0)
  (`PrimitiveComponent.SetSimulatePhysics` (`self.Body`) false))

(fn `UserConstructionScript`)