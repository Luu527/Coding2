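; BP_Door is a hinged door that opens for the third-person character only when it holds at least one key.
; Entering the box trigger checks the character's TotalKeys, then either plays the DoorRotate timeline to swing the mesh's yaw open or prints a locked message.
; When the character leaves the box, the timeline reverses to close the door.
; Keys are only checked, not consumed, and debug strings report each result.
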(event `self.ReceiveBeginPlay`)

(event `self.Box.OnComponentBeginOverlap`
  (params (OverlappedComponent :type "PrimitiveComponent Object Reference") (OtherActor :type "Actor Object Reference") (OtherComp :type "PrimitiveComponent Object Reference") (OtherBodyIndex :type Integer) (bFromSweep :type Boolean) (SweepResult :type "HitResult Structure (by ref)"))
  (`KismetSystemLibrary.PrintString` "Here's a door")
  (bind _asbp_third_person_character (cast `/Game/ThirdPerson/Blueprints/BP_ThirdPersonCharacter` OtherActor))
  (if (> (`/Game/ThirdPerson/Blueprints/BP_ThirdPersonCharacter.totalKeys` _asbp_third_person_character) 0)
    (`KismetSystemLibrary.PrintString` "Key> 0, Door OPEN" true true (struct :`R` 0.21303 :`G` 1.0 :`B` 0.496732 :`A` 1.0) 3.0)
    (bind (_direction _newtrack_0) (`Timeline|DoorRotate` :!label _label)
      (:`Update`
        (`SceneComponent.K2_SetRelativeRotation` (`self.hinged_door3_LOD0`) (`KismetMathLibrary.MakeRotator` 0.0 0.0 (`KismetMathLibrary.Lerp` 0.0 -90.0 _newtrack_0)) false false)))
    (else
      (`KismetSystemLibrary.PrintString` "Key<1 , Door LOCKED" true true (struct :`R` 1.0 :`G` 0.05221 :`B` 0.074176 :`A` 1.0) 3.0))))

(event `self.Box.OnComponentEndOverlap`
  (params (OverlappedComponent :type "PrimitiveComponent Object Reference") (OtherActor :type "Actor Object Reference") (OtherComp :type "PrimitiveComponent Object Reference") (OtherBodyIndex :type Integer))
  (cast `/Game/ThirdPerson/Blueprints/BP_ThirdPersonCharacter` OtherActor)
  (goto _label :!via `Reverse`))

(fn `UserConstructionScript`)