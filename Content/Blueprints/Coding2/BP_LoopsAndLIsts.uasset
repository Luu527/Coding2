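; Practice Blueprint demonstrating loops and arrays through on-screen debug printing.
; BeginPlay starts DelayLoop, a self-calling event that prints and increments a counter, waits half a second, runs PrintColors, then repeats endlessly.
; PrintColors shuffles the TextColors array and prints each index in its color, followed by a completion message.
; A few random-pick and color-array nodes are left unused.
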(event `self.ReceiveBeginPlay`
  (`KismetSystemLibrary.PrintString` "loops and list is active" true true (struct :`R` 0.160093 :`G` 0.321873 :`B` 1.0 :`A` 1.0) 5.0)
  (`self.Delay Loop`))

(event `Delay Loop`
  (`KismetSystemLibrary.PrintString` (`KismetStringLibrary.Concat_StrStr` "StartingDelayLoop# " (`KismetStringLibrary.Conv_IntToString` (`self.DelayLoopCounter`))))
  (`/Engine/EditorBlueprintResources/StandardMacros.IncrementInt` (`self.DelayLoopCounter`)
    (:`  `
      (`KismetSystemLibrary.Delay` 0.5)
      (`self.PrintColors`)
      (`self.Delay Loop`))))

(event `PrintColors`
  (bind _textcolors (`self.TextColors`))
  (`KismetArrayLibrary.Array_Shuffle` _textcolors)
  (for (_array_element _array_index) _textcolors
    (`KismetSystemLibrary.PrintString` (`KismetStringLibrary.Concat_StrStr` "printingColor" (`KismetStringLibrary.Conv_IntToString` _array_index)) true true _array_element))
  (`KismetSystemLibrary.PrintString` "We are done printing colors" true true (struct :`R` 1.0 :`G` 0.075322 :`A` 1.0)))

(fn `UserConstructionScript`)