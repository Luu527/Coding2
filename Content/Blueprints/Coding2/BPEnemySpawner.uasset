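; Enemy spawner that creates a randomized BP_AiMoveTo enemy at every BP_enemySpawnPoint in the level on BeginPlay.
; Each spawn draws a random name, head/legs material, torso material and skeletal mesh from the spawner's arrays.
; The name is re-rolled when set after spawning and again for the debug print, so the printed name can differ from the assigned one.
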(event `self.ReceiveBeginPlay`
  (bind _output (`|GetArrayItem` (`self.EnemyNames`) (`KismetMathLibrary.RandomIntegerInRange` 0 (- (`KismetArrayLibrary.Array_Length` (`self.EnemyNames`)) 1))))
  (`KismetSystemLibrary.PrintString` "enemySpawner is active" true true (struct :`R` 1.0 :`G` 0.091599 :`A` 1.0) 5.0)
  (bind _outactors (`GameplayStatics.GetAllActorsOfClass` "/Game/Blueprints/Coding2/BP_enemySpawnPoint.BP_enemySpawnPoint_C"))
  (for _array_element _outactors
    (bind _returnvalue (`|SpawnActorFromClass` "/Game/AI_Blueprints/BP_AiMoveTo.BP_AiMoveTo_C" (`self.GetTransform` _array_element) "Undefined" "MultiplyWithRoot" null _output (`|GetArrayItem` (`self.EnemyMaterials`) (`KismetMathLibrary.RandomIntegerInRange` 0 (- (`KismetArrayLibrary.Array_Length` (`self.EnemyMaterials`)) 1))) (`|GetArrayItem` (`self.EnemyMaterials`) (`KismetMathLibrary.RandomIntegerInRange` 0 (- (`KismetArrayLibrary.Array_Length` (`self.EnemyMaterials`)) 1))) (`|GetArrayItem` (`self.EnemySkeletalMeshes`) (`KismetMathLibrary.RandomIntegerInRange` 0 (- (`KismetArrayLibrary.Array_Length` (`self.EnemySkeletalMeshes`)) 1))) null))
    (set `/Game/AI_Blueprints/BP_AiMoveTo.EnemyName` _output _returnvalue)
    (`KismetSystemLibrary.PrintString` (`KismetStringLibrary.Concat_StrStr` "Enemy " _output " is spawned") true true (struct :`G` 0.66 :`B` 1.0 :`A` 1.0) 5.0)))

(fn `UserConstructionScript`)