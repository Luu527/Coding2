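; Game mode that saves and loads the player's stats through an SG_PlayerStats save game in the "Player Save" slot.
; On BeginPlay it loads the slot and copies Stamina onto the player's BP_ThirdPersonCharacter, or creates a new save object if none exists.
; SavePlayerStats writes the held save object to the slot and prints the result, without reading values from the character itself.
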(event `self.ReceiveBeginPlay`
  (`KismetSystemLibrary.PrintString` "Loading theSaveLoad Game Mode" true true (struct :`R` 1.0 :`G` 0.05221 :`B` 0.074176 :`A` 1.0) 10.0)
  (`self.Load Player Stats`))

(event `Load Player Stats`
  (bind _returnvalue (`GameplayStatics.DoesSaveGameExist` "Player Save"))
  (if _returnvalue
    (bind _returnvalue_2 (`GameplayStatics.LoadGameFromSlot` "Player Save"))
    (bind _assg_player_stats (cast `/Game/Blueprints/SavingLoading/SG_PlayerStats` _returnvalue_2))
    (set `self.SG_PLayerStats` _assg_player_stats)
    (bind _asbp_third_person_character (cast `/Game/ThirdPerson/Blueprints/BP_ThirdPersonCharacter` (`GameplayStatics.GetPlayerCharacter` 0)))
    (set `/Game/ThirdPerson/Blueprints/BP_ThirdPersonCharacter.Stamina` (`/Game/Blueprints/SavingLoading/SG_PlayerStats.Stamina` (`self.SG_PLayerStats`)) _asbp_third_person_character)
    (`KismetSystemLibrary.PrintString` "Player Stats has been loaded" true true (struct :`R` 0.48497 :`G` 0.287625 :`B` 0.800347 :`A` 1.0) 5.0)
    (else
      (bind _returnvalue_3 (`GameplayStatics.CreateSaveGameObject` "/Game/Blueprints/SavingLoading/SG_PlayerStats.SG_PlayerStats_C"))
      (set `self.SG_PLayerStats` _returnvalue_3))))

(event `Save Player Stats`
  (bind _returnvalue (`GameplayStatics.SaveGameToSlot` (`self.SG_PLayerStats`) "Player Save"))
  (if _returnvalue
    (`KismetSystemLibrary.PrintText` "Player Stats written to Save Game file" true true (struct :`R` 0.275057 :`G` 1.0 :`B` 0.674974 :`A` 1.0) 5.0)
    (else
      (`KismetSystemLibrary.PrintText` "Player Stats could not written to Save Game file" true true (struct :`R` 1.0 :`G` 0.075322 :`A` 1.0) 5.0))))

(fn `UserConstructionScript`)