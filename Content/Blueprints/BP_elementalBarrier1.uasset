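; BP_elementalBarrier1 is an elemental barrier that kills the third-person player character on overlap unless the character's elemental immunity matches its type.
; On BeginPlay it switches on its ElementalType to set a text label naming the barrier's element and prints the type.
; The cube's overlap event casts to the character, compares immunity, and on a mismatch prints a death message and quits the game after a short delay.
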(event `self.ReceiveBeginPlay`
  (`KismetSystemLibrary.PrintText` (`|GenericToText` (`self.ElementalType`)))
  (switch `/Game/Blueprints/Enumeration/ElementalTpye` (`self.ElementalType`)
    (:`NewEnumerator1`
      (`TextRenderComponent.K2_SetText` (`self.TextRender`) "Barrier Of Fire"))
    (:`NewEnumerator2`
      (`TextRenderComponent.K2_SetText` (`self.TextRender`) "Barrier Of water"))
    (:`NewEnumerator3`
      (`TextRenderComponent.K2_SetText` (`self.TextRender`) "Barrier Of Earth"))
    (:`NewEnumerator4`
      (`TextRenderComponent.K2_SetText` (`self.TextRender`) "Barrier Of Air"))
    (:`NewEnumerator5`
      (`TextRenderComponent.K2_SetText` (`self.TextRender`) "Barrier Of Poison"))
    (:`NewEnumerator6`
      (`TextRenderComponent.K2_SetText` (`self.TextRender`) "Barrier Of Void"))))

(event `self.Cube.OnComponentBeginOverlap`
  (params (OverlappedComponent :type "PrimitiveComponent Object Reference") (OtherActor :type "Actor Object Reference") (OtherComp :type "PrimitiveComponent Object Reference") (OtherBodyIndex :type Integer) (bFromSweep :type Boolean) (SweepResult :type "HitResult Structure (by ref)"))
  (bind _asbp_third_person_character (cast `/Game/ThirdPerson/Blueprints/BP_ThirdPersonCharacter` OtherActor))
  (if (not (`|EnumEquality` (`/Game/ThirdPerson/Blueprints/BP_ThirdPersonCharacter.Elemental Immunety` _asbp_third_person_character) (`self.ElementalType`)))
    (`KismetSystemLibrary.PrintString` "You are Died")
    (`KismetSystemLibrary.Delay` 2.0)
    (`KismetSystemLibrary.QuitGame` null "Quit")))

(fn `UserConstructionScript`)