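; BP_AiMoveTo is an AI pawn with a configurable mesh and a floating name that follows the player.
; On BeginPlay it applies its skeletal mesh and head/legs and torso materials, then writes EnemyName into its W_EnemyName widget.
; It then repeatedly calls AIMoveTo toward player controller 0 (not the pawn), retrying one second after each success or failure.
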(event `self.ReceiveBeginPlay`
  (`SkeletalMeshComponent.SetSkeletalMeshAsset` (`self.Mesh`) (`self.InitialSkeletalMesh`))
  (`PrimitiveComponent.SetMaterial` (`self.Mesh`) 0 (`self.HeadLegsMaterial`))
  (`PrimitiveComponent.SetMaterial` (`self.Mesh`) 1 (`self.TorsoMaterial`))
  (`|ExecutionSequence`
    (:`then_0`
      (bind _asw_enemy_name (cast `/Game/Blueprints/Coding2/W_EnemyName` (`WidgetComponent.GetUserWidgetObject` (`self.NameWidget`))))
      (set `TextBlock.Text` (`KismetTextLibrary.Conv_StringToText` (`self.EnemyName`)) (`/Game/Blueprints/Coding2/W_EnemyName.NameText` _asw_enemy_name))
      (`KismetSystemLibrary.PrintString` "set name is active" true true (struct :`G` 0.66 :`B` 1.0 :`A` 1.0) 5.0))
    (:`then_1`
      (`|AIMoveTo` self (0.0 0.0 0.0) (`GameplayStatics.GetPlayerController` 0) 200.0 :!label _label
        (:`OnSuccess`
          _)
        (:`OnFail`
          _))
      (`KismetSystemLibrary.Delay` 1.0)
      (goto _label))))

(fn `UserConstructionScript`)